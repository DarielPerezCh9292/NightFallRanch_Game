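; Inventory actor Blueprint that outlines a slot-based item container, still largely unimplemented.
; BeginPlay pads the Slots array up to MaxSlots by setting its last index with size-to-fit.
; PickUpSlot is an unfinished draft with an empty loop over Slots and unconnected type-matching nodes.
; Drag, drop, get, receive, return, send, throw and use slot functions are empty stubs.
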(event `self.ReceiveBeginPlay`
  (if (< (`KismetArrayLibrary.Array_Length` (`self.Slots`)) (`self.MaxSlots`))
    (`KismetArrayLibrary.Array_Set` (`self.Slots`) (- (`self.MaxSlots`) 1) (struct) true)))

(fn `DragSlot`
  (params (Index :type Integer) (Amount :type Integer)))

(fn `DropSlot`
  (params (Index :type Integer)))

(fn `GetInventorySlot`)

(fn `PickUpSlot`
  (params (Slot :type "/Game/Dynamic/Items/Base/Structures/InventorySlotStructure Structure"))
  (returns (Return :type Boolean) (AmountLeft :type Integer))
  (locals (Added :type Boolean) (Proxy :type "/Game/Dynamic/Items/Base/Structures/InventorySlotStructure Structure") (SavedAmount :type Integer) (SavedAmountProxy :type Integer))
  (bind _output_get (set `local.Proxy` Slot))
  (set `local.SavedAmount` (`.Amount_9_A32D53B9468913E6C4187BA48865B0CC` (break `/Game/Dynamic/Items/Base/Structures/InventorySlotStructure` _output_get)))
  (for _array_element (`self.Slots`)
    _)
  (if (and (> (`local.SavedAmount`) 0) (`local.Added`))
    (set `local.Added` true)
    (elif (`local.Added`)
      (return true 0))))

(fn `ReceiveSlot`
  (params (Index :type Integer) (Slot :type "/Game/Dynamic/Items/Base/Structures/InventorySlotStructure Structure")))

(fn `ReturnSlot`)

(fn `SendSlot`
  (params (To :type "Object Object Reference") (Index :type Integer)))

(fn `ThrowSlot`
  (params (Location :type "Vector Structure") (Vector :type "Vector Structure")))

(fn `UserConstructionScript`)

(fn `UseSlot`
  (params (Index :type Integer)))